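; Game state for a match with Monster and Human roles, handling a ready check and player spawning.
; LaunchGame counts ready BP_PlayerStates, resetting the count unless it equals two; no launch action follows yet.
; SpawnPlayer finds PlayerStarts tagged with the requested type, spawns BP_Monster or FirstPersonCharacter there, and has the given controller possess it.
; The loop has no break, so every matching start spawns a pawn.
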(event Custom|LaunchGame
  (bind _array_element (Utilities|Array|ForEachLoopwithBreak (Variables|Default|GetPlayerArray))
    (:LoopBody
      (if (Variables|/Game/Blueprints/BP_PlayerState.BP_PlayerState_C|GetReady? (.AsBP%20Player%20State (Utilities|Casting|CastToBP_PlayerState _array_element)))
        (Math|Integer|IncrementInt (Variables|Default|GetCount))))
    (:Completed
      (if (not (== (Variables|Default|GetCount) 2))
        (Variables|Default|SetCount 0)))))

(event Custom|SpawnPlayer
  (params (PlayerController :type BP%20Player%20Controller%20Object%20Reference) (Type :type Name))
  (Development|PrintString "SpawnPlayer" true true "(R=0.000000,G=0.660000,B=1.000000,A=1.000000)" 2e+01)
  (bind _outactors (Actor|GetAllActorsOfClass "/Script/Engine.PlayerStart"))
  (for _array_element _outactors
    (if (Utilities|Name|Equal(Name) (Variables|/Script/Engine.PlayerStart|GetPlayerStartTag _array_element) Type)
      (switch name Type
        (:Monster
          (bind _returnvalue (Game|SpawnActorfromClass "/Game/Monster/Blueprints/BP_Monster.BP_Monster_C" (Transformation|GetActorTransform _array_element) "Undefined" 0 0))
          (Pawn|Possess PlayerController _returnvalue))
        (:Human
          (bind _returnvalue_2 (Game|SpawnActorfromClass "/Game/FirstPersonBP/Blueprints/FirstPersonCharacter.FirstPersonCharacter_C" (Transformation|GetActorTransform _array_element) "Undefined" 0 0))
          (Pawn|Possess PlayerController _returnvalue_2))))))

(event EventBeginPlay)

(event EventTick
  (params (DeltaSeconds :type Float%20%28single-precision%29)))

(fn ConstructionScript)